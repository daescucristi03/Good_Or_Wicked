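; First-person player character with walk, smoothly interpolated sprint, jump, look, and physics-based object pickup.
; Interactables register and unregister themselves through events into a list.
; Each tick it highlights the registered item most aligned with the camera forward vector, using a dot-product threshold.
; Holding Interact grabs the highlighted mesh with a physics handle, which follows a pickup position until release.
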(event `InputAction|Jump`
  (params (Key :type "Key Structure"))
  ;[1 0 0.3984] Movement
  (:`Pressed`
    (`self.Jump`))
  (:`Released`
    (`self.StopJumping`)))

(event `/Game/Blueprints/Interfaces/BPI_Interact.RegisterInteractable`
  (params (Interactable :type "/Game/Blueprints/Objects/BP_Base_Interactable Object Reference"))
  (`self.HandleRegisterInteractable` Interactable))

(event `InputAxis|MoveForward`
  (params (AxisValue :type "Float (single-precision)"))
  ;[1 0 0.3984] Movement
  (set `self.Vertical_Input` AxisValue))

(event `/Game/Blueprints/Interfaces/BPI_Interact.UnregisterInteractable`
  (params (Interactable :type "/Game/Blueprints/Objects/BP_Base_Interactable Object Reference"))
  (`self.HandleUnregisterInteractable` Interactable))

(event `InputAxis|MoveRight`
  (params (AxisValue :type "Float (single-precision)"))
  ;[1 0 0.3984] Movement
  (set `self.Horizontal_Input` AxisValue))

(event `InputAxis|LookUp`
  (params (AxisValue :type "Float (single-precision)"))
  ;[1 0 0.3984] Movement
  (`self.AddControllerPitchInput` AxisValue))

(event `InputAction|Sprint`
  (params (Key :type "Key Structure"))
  ;[1 0 0.3984] Movement
  (:`Pressed`
    (set `self.isSprinting` true))
  (:`Released`
    (set `self.isSprinting` false)))

(event `InputAxis|Turn`
  (params (AxisValue :type "Float (single-precision)"))
  ;[1 0 0.3984] Movement
  (`self.AddControllerYawInput` AxisValue))

(event `self.ReceiveTick`
  (params (DeltaSeconds :type "Float (single-precision)"))
  ;[0 1 0.7188] Event Tick
  (`self.Movement`)
  (`self.Sprint`)
  (`self.UpdateBestInteractable`)
  (`self.UpdateGrabPosition`))

(event `InputAction|Interact`
  (params (Key :type "Key Structure"))
  (:`Pressed`
    (`self.PickUp`))
  (:`Released`
    (`self.Drop`)))

(event `PickUp`
  (`/Engine/EditorBlueprintResources/StandardMacros.IsValid` (`self.HighlightedInteractable`)
    (:`Is Valid`
      (`PhysicsHandleComponent.GrabComponentAtLocation` (`self.PhysicsHandle`) (`/Game/Blueprints/Objects/BP_Base_Interactable.Mesh` (`self.HighlightedInteractable`)) "None" (`SceneComponent.K2_GetComponentLocation` (`self.PickUp_Position`))))))

(event `Drop`
  (`PhysicsHandleComponent.ReleaseComponent` (`self.PhysicsHandle`)))

(event `UpdateGrabPosition`
  (`PhysicsHandleComponent.SetTargetLocation` (`self.PhysicsHandle`) (`SceneComponent.K2_GetComponentLocation` (`self.PickUp_Position`))))

(fn `GetBestInteractable`
  (locals (InteractableVariables :type "/Game/Blueprints/Structs/F_Interactable_Variables Structure"))
  (bind (_interactablevariables_dot _interactablevariables_interactable) (break `/Game/Blueprints/Structs/F_Interactable_Variables` (`local.InteractableVariables`)))
  (bind _camera (`self.Camera`))
  (bind _interactablevariables_dot_2 (break `/Game/Blueprints/Structs/F_Interactable_Variables` (`local.InteractableVariables`)))
  (set `local.InteractableVariables` (make `/Game/Blueprints/Structs/F_Interactable_Variables` -1.0))
  (for _array_element (`self.Interactables`)
    (bind _returnvalue (`KismetMathLibrary.Dot_VectorVector` (`KismetMathLibrary.Normal` (- (`PrimitiveComponent.GetCenterOfMass` (`/Game/Blueprints/Objects/BP_Base_Interactable.Mesh` _array_element) "None") (`SceneComponent.K2_GetComponentLocation` _camera))) (`SceneComponent.GetForwardVector` _camera)))
    (if (and (> _returnvalue 0.8) (> _returnvalue _interactablevariables_dot_2))
      (set `local.InteractableVariables` (make `/Game/Blueprints/Structs/F_Interactable_Variables` _returnvalue _array_element))))
  (`/Engine/EditorBlueprintResources/StandardMacros.IsValid` _interactablevariables_interactable
    (:`Is Valid`
      (`self.SetBestInteractable` _interactablevariables_interactable))
    (:`Is Not Valid`
      (`self.SetBestInteractable` null))))

(fn `HandleRegisterInteractable`
  (params (Interactable :type "/Game/Blueprints/Objects/BP_Base_Interactable Object Reference"))
  (`KismetArrayLibrary.Array_AddUnique` (`self.Interactables`) Interactable))

(fn `HandleUnregisterInteractable`
  (params (Interactable :type "/Game/Blueprints/Objects/BP_Base_Interactable Object Reference"))
  (`KismetArrayLibrary.Array_RemoveItem` (`self.Interactables`) Interactable))

(fn `Movement`
  (`|ExecutionSequence`
    (:`then_0`
      (`self.AddMovementInput` (`KismetMathLibrary.GetForwardVector` (`self.K2_GetActorRotation`)) (`self.Vertical_Input`)))
    (:`then_1`
      (`self.AddMovementInput` (`KismetMathLibrary.GetRightVector` (`self.K2_GetActorRotation`)) (`self.Horizontal_Input`)))))

(fn `SetBestInteractable`
  (params (Interactable :type "/Game/Blueprints/Objects/BP_Base_Interactable Object Reference"))
  (`/Engine/EditorBlueprintResources/StandardMacros.IsValid` Interactable
    (:`Is Valid`
      (if (!= Interactable (`self.HighlightedInteractable`))
        (bind _highlightedinteractable (`self.HighlightedInteractable`)
          (:`then`
            (`/Game/Blueprints/Objects/BP_Base_Interactable.SetHighlight` _highlightedinteractable false))
          (:`else`
            _)))
      (bind _output_get (set `self.HighlightedInteractable` Interactable))
      (`/Game/Blueprints/Objects/BP_Base_Interactable.SetHighlight` _output_get true))
    (:`Is Not Valid`
      (bind _highlightedinteractable_2 (`self.HighlightedInteractable`)
        (:`then`
          (`/Game/Blueprints/Objects/BP_Base_Interactable.SetHighlight` _highlightedinteractable_2 false)
          (set `self.HighlightedInteractable` null))
        (:`else`)))))

(fn `Sprint`
  (if (`self.isSprinting`)
    (set `CharacterMovementComponent.MaxWalkSpeed` (`KismetMathLibrary.FInterpTo_Constant` (`CharacterMovementComponent.MaxWalkSpeed` (`self.CharacterMovement`)) 600.0 (`GameplayStatics.GetWorldDeltaSeconds`) 600.0) (`self.CharacterMovement`))
    (else
      (set `CharacterMovementComponent.MaxWalkSpeed` (`KismetMathLibrary.FInterpTo_Constant` (`CharacterMovementComponent.MaxWalkSpeed` (`self.CharacterMovement`)) 300.0 (`GameplayStatics.GetWorldDeltaSeconds`) 600.0) (`self.CharacterMovement`)))))

(fn `UpdateBestInteractable`
  (if (> (`KismetArrayLibrary.Array_Length` (`self.Interactables`)) 0)
    (`self.GetBestInteractable`)
    (else
      (`self.SetBestInteractable` null))))

(fn `UserConstructionScript`)